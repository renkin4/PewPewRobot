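; MySaveInfo is a save data container for the player's name and audio settings: music and SFX volume plus their mute states.
; The InitializeSaveData event copies its five inputs into the matching variables.
; GetAllData returns all five stored values in one call.
; The asset only holds the data; neither graph performs saving or loading to a slot.
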(event `InitializeSaveData`
  (params (PlayerName :type String) (MusicVolume :type "Float (double-precision)") (SFXVolume :type "Float (double-precision)") (bIsMusicMuted :type Boolean) (bIsSFXMuted :type Boolean))
  (`|ExecutionSequence`
    (:`then_0`
      (set `self.PlayerName` PlayerName))
    (:`then_1`
      (set `self.MusicVolume` MusicVolume))
    (:`then_2`
      (set `self.SFXVolume` SFXVolume))
    (:`then_3`
      (set `self.bIsMusicMuted` bIsMusicMuted))
    (:`then_4`
      (set `self.bIsSFXMuted` bIsSFXMuted))))

(fn `GetAllData`
  (returns (PlayerName :type String) (MusicVolume :type "Float (double-precision)") (SFXVolume :type "Float (double-precision)") (bIsMusicMuted :type Boolean) (bIsSFXMuted :type Boolean))
  (return (`self.PlayerName`) (`self.MusicVolume`) (`self.SFXVolume`) (`self.bIsMusicMuted`) (`self.bIsSFXMuted`)))