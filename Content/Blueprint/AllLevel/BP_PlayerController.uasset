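; Player controller that owns the local player's UI: lobby, score, health, aiming cursor and shop widgets.
; On the local authority it shows a lobby whose Start button tells BP_GameplayGM to start the match.
; The score widget waits on a retry loop for a valid PlayerState.
; Possession sets CharacterRef, whose OnRep rebuilds the health widget, and calls a client event for game input and the cursor, which Tick shows while aiming.
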(event `OnClickStartGame`
  ;[1 1 1] Temporary
  (if (`self.IsLocalPlayerController`)
    (set `self.bShowMouseCursor` false)
    (`WidgetBlueprintLibrary.SetFocusToGameViewport`)
    (`WidgetBlueprintLibrary.SetInputMode_GameOnly` self)
    (`Widget.SetVisibility` (`self.LobbyWidgetRef`) "Hidden")
    (bind _asbp_gameplay_gm (cast `/Game/Blueprint/AllLevel/BP_GameplayGM` (`GameplayStatics.GetGameMode`)))
    (`MyGameMode_Base.SetShouldStartMatch` _asbp_gameplay_gm true)))

(event `self.ReceiveBeginPlay`
  (bind _lobbywidgetref (`self.LobbyWidgetRef`))
  ;[1 1 1] Temporary
  (`parent.ReceiveBeginPlay`)
  (if (`self.IsLocalPlayerController`)
    (`|ExecutionSequence`
      (:`then_0`
        (`/Engine/EditorBlueprintResources/ActorMacros.Switch Has Authority`
          (:`Authority`
            (`WidgetBlueprintLibrary.SetFocusToGameViewport`)
            (bind _returnvalue (`|CreateWidget` "/Game/UI/Lobby/Lobby_Widget.Lobby_Widget_C"))
            (bind _output_get (set `self.LobbyWidgetRef` _returnvalue))
            (`UserWidget.AddToViewport` _output_get 0)
            (set `self.bShowMouseCursor` true)
            (`WidgetBlueprintLibrary.SetInputMode_UIOnlyEx` self _lobbywidgetref)
            (add `Button.OnClicked` (`/Game/UI/Lobby/Lobby_Widget.StartGame` _lobbywidgetref) (delegate `OnClickStartGame`)))))
      (:`then_1`
        (bind _playerstate (`self.PlayerState` :!label _label)
          (:`then`
            (bind _asbp_player_state (cast `/Game/Blueprint/AllLevel/BP_PlayerState` _playerstate))
            (bind _returnvalue_2 (`|CreateWidget` "/Game/UI/Gameplay/Score_Widget.Score_Widget_C" null _asbp_player_state))
            (`UserWidget.AddToViewport` _returnvalue_2 0))
          (:`else`
            (`KismetSystemLibrary.Delay` 0.5)
            (goto _label)))))))

(event `self.OnPossessEvent`
  (params (InPawn :type "Pawn Object Reference"))
  (`parent.OnPossessEvent` InPawn)
  (bind _asbp_character (cast `/Game/Blueprint/Gameplay/Character/BP_Character` InPawn))
  (set `self.CharacterRef` _asbp_character)
  (`self.CLIENT_SetInputFocus`))

(event `self.ReceiveTick`
  (params (DeltaSeconds :type "Float (single-precision)"))
  (bind _cursor (`self.Cursor`))
  ;[1 1 1] Cursor UI Need to refactor
  (`parent.ReceiveTick` DeltaSeconds)
  (`/Engine/EditorBlueprintResources/StandardMacros.IsValid` _cursor
    (:`Is Valid`
      (if (`self.GetIsAiming`)
        (`Widget.SetVisibility` _cursor "Visible")
        (else
          (`Widget.SetVisibility` _cursor "Hidden"))))))

(event `CLIENT_SetInputFocus`
  (`|ExecutionSequence`
    (:`then_0`
      (`WidgetBlueprintLibrary.SetFocusToGameViewport`)
      (`WidgetBlueprintLibrary.SetInputMode_GameOnly` self))
    (:`then_1`
      ;[1 1 1] Refactor To HUd
      (bind _returnvalue (`|CreateWidget` "/Game/UI/Gameplay/Cursor_Widget.Cursor_Widget_C" self))
      (bind _output_get (set `self.Cursor` _returnvalue))
      (`UserWidget.AddToViewport` _output_get 0)
      (`Widget.SetVisibility` (`self.Cursor`) "Hidden"))))

(fn `CreateShopUI`
  (params (ItemToSell :type "Array of Actor Class Reference"))
  (returns (ShopWidgetRef :type "/Game/UI/Gameplay/Shop_Widget Object Reference"))
  (if (`self.IsLocalController`)
    (`self.ShopWidgetRef`
      (:`then`)
      (:`else`
        (bind _returnvalue (`|CreateWidget` "/Game/UI/Gameplay/Shop_Widget.Shop_Widget_C" null ItemToSell))
        (set `self.ShopWidgetRef` _returnvalue)
        (`UserWidget.AddToViewport` _returnvalue 0)
        (return (`self.ShopWidgetRef`))))))

(fn `OnRep_CharacterRef`
  (if (`self.IsLocalPlayerController`)
    (`self.WrapperWidget`
      (:`then`
        (`Widget.RemoveFromParent` (`self.WrapperWidget`)))
      (:`else`
        _))
    (bind _returnvalue (`|CreateWidget` "/Game/UI/Gameplay/Widget_Health.Widget_Health_C" null (`self.CharacterRef`)))
    (bind _output_get (set `self.WrapperWidget` _returnvalue))
    (`UserWidget.AddToViewport` _output_get 0)))

(fn `UserConstructionScript`)