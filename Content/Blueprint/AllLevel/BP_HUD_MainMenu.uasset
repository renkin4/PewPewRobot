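; Main menu HUD that draws a full-screen background texture and switches between the first selection, host game, join server and options screens.
; Each Create function clears all widgets, then creates its widget on first use and reuses it afterwards.
; BeginPlay opens the first selection screen, retrying until the game instance cast succeeds.
; It then applies saved SFX and music volumes through sound mixes and starts the menu music if a save loads.
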(event `self.ReceiveBeginPlay`
  (`self.CreateFirstSelection`)
  (bind _asbp_game_instance (cast `/Game/Blueprint/AllLevel/System/BP_GameInstance` (`GameplayStatics.GetGameInstance`) :!label _label)
    (:`then`
      (bind _savegamedata (`/Game/Blueprint/AllLevel/System/BP_GameInstance.LoadGame` _asbp_game_instance))
      (`/Engine/EditorBlueprintResources/StandardMacros.IsValid` _savegamedata
        (:`Is Valid`
          (bind _asmy_save_info (cast `/Game/Blueprint/AllLevel/System/MySaveInfo` _savegamedata))
          (`|ExecutionSequence`
            (:`then_0`
              (`GameplayStatics.SetSoundMixClassOverride` "/Game/Blueprint/Gameplay/Sound/SFX_SoundMixer.SFX_SoundMixer" "/Game/Blueprint/Gameplay/Sound/SFX_SoundClass.SFX_SoundClass" (`/Game/Blueprint/AllLevel/System/MySaveInfo.SFXVolume` _asmy_save_info))
              (`GameplayStatics.PushSoundMixModifier` "/Game/Blueprint/Gameplay/Sound/SFX_SoundMixer.SFX_SoundMixer"))
            (:`then_1`
              (`GameplayStatics.SetSoundMixClassOverride` "/Game/Blueprint/Gameplay/Sound/Music_SoundMixer.Music_SoundMixer" "/Game/Blueprint/Gameplay/Sound/Music_SoundClass.Music_SoundClass" (`/Game/Blueprint/AllLevel/System/MySaveInfo.MusicVolume` _asmy_save_info))
              (`GameplayStatics.PushSoundMixModifier` "/Game/Blueprint/Gameplay/Sound/Music_SoundMixer.Music_SoundMixer")
              (`GameplayStatics.PlaySound2D` "/Game/Asset/Sound/A-City-for-All-Mankind_Cue.A-City-for-All-Mankind_Cue"))))))
    (:`CastFailed`
      (`KismetSystemLibrary.Delay` 0.2)
      (goto _label))))

(event `self.ReceiveDrawHUD`
  (params (SizeX :type Integer) (SizeY :type Integer))
  (bind (_screendimension_x _screendimension_y) (`KismetMathLibrary.BreakVector2D` (`self.ScreenDimension`)))
  (set `self.ScreenDimension` (`KismetMathLibrary.MakeVector2D` (`KismetMathLibrary.Conv_IntToDouble` SizeX) (`KismetMathLibrary.Conv_IntToDouble` SizeY)))
  (`self.DrawTexture` "/Game/Asset/UI/PNG/BACKGROUND.BACKGROUND" 0.0 0.0 _screendimension_x _screendimension_y 1.0 1.0 1.0 1.0))

(fn `CreateFirstSelection`
  (bind _firstselectionwidget (`self.FirstSelectionWidget`))
  (`WidgetLayoutLibrary.RemoveAllWidgets`)
  (`self.FirstSelectionWidget`
    (:`then`
      _)
    (:`else`
      (bind _returnvalue (`|CreateWidget` "/Game/UI/Menu/W_MenuFirstSelection.W_MenuFirstSelection_C"))
      (set `self.FirstSelectionWidget` _returnvalue)))
  (`UserWidget.AddToViewport` (`self.FirstSelectionWidget`) 0)
  (`UserWidget.SetAnchorsInViewport` _firstselectionwidget (make `Anchors` (0.5 0.5) (0.5 0.5)))
  (`UserWidget.SetAlignmentInViewport` _firstselectionwidget (0.5 -0.26)))

(fn `CreateHostGame`
  (`WidgetLayoutLibrary.RemoveAllWidgets`)
  (`self.HostGameWidget`
    (:`then`
      _)
    (:`else`
      (bind _returnvalue (`|CreateWidget` "/Game/UI/Menu/W_HostGame.W_HostGame_C"))
      (set `self.HostGameWidget` _returnvalue)))
  (`UserWidget.AddToViewport` (`self.HostGameWidget`) 0))

(fn `CreateJoinServer`
  (`WidgetLayoutLibrary.RemoveAllWidgets`)
  (`self.JoinGameWidget`
    (:`then`
      _)
    (:`else`
      (bind _returnvalue (`|CreateWidget` "/Game/UI/Menu/W_joinGame.W_JoinGame_C"))
      (set `self.JoinGameWidget` _returnvalue)))
  (`UserWidget.AddToViewport` (`self.JoinGameWidget`) 0))

(fn `CreateMenuOption`
  (`WidgetLayoutLibrary.RemoveAllWidgets`)
  (`self.MenuOptionWidget`
    (:`then`
      _)
    (:`else`
      (bind _returnvalue (`|CreateWidget` "/Game/UI/Menu/W_MenuOption.W_MenuOption_C"))
      (set `self.MenuOptionWidget` _returnvalue)))
  (`UserWidget.AddToViewport` (`self.MenuOptionWidget`) 0))

(fn `UserConstructionScript`)