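; Gameplay game mode that resets global time dilation to normal on begin play, after running the parent logic.
; Overrides the spawn color change by calling the parent with a yellow material.
; Defines an event that spawns a batch of score boxes at random navigable points around the map origin.
; The looping timer and initial call for that box spawning are disconnected, so neither runs here.
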(event `self.ReceiveBeginPlay`
  (`parent.ReceiveBeginPlay`)
  (`GameplayStatics.SetGlobalTimeDilation` 1.0))

(event `SpawnBoxesTimer`
  (for _ (range 4)
    (`self.SpawnBox` "/Game/Blueprint/Gameplay/Box/BP_ScoreBox.BP_ScoreBox_C" (`NavigationSystem.K2_GetRandomLocationInNavigableRadius` (`KismetMathLibrary.MakeVector` 0.0 0.0 10.0) 750.0 null "/Script/Engine.RecastFilter_UseDefaultArea"))))

(event `self.ChangeSpawnColor`
  (params (PState :type "PlayerState_Base Object Reference") (MaterialInterface :type "MaterialInterface Object Reference"))
  (`parent.ChangeSpawnColor` PState "/Game/Asset/Temp/Yellow.Yellow"))

(fn `UserConstructionScript`)