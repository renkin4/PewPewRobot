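; Multiplayer player controller that links each player to the HUD, shop and character inventory.
; BeginPlay initializes lobby UI and retries score setup until PlayerState is valid; CharacterRef's OnRep initializes the player HUD.
; Possession triggers client game-only input and creates a cursor widget, which Tick shows while aiming.
; Server events add inventory items and handle purchases, with BuyItem routing to authority to spawn weapons through the GameMode and attach them.
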(event `self.ReceiveBeginPlay`
  ;[1 1 1] Initialize UIs
  (`parent.ReceiveBeginPlay`)
  (bind _asbp_hud (cast `/Game/Blueprint/Gameplay/BP_HUD` (`self.GetHUD`)))
  (set `self.HUDRef` _asbp_hud)
  (`|ExecutionSequence`
    (:`then_0`
      (`/Game/Blueprint/Gameplay/BP_HUD.Initializelobby` (`self.HUDRef`) (`KismetSystemLibrary.IsServer`))
      (set `self.bShowMouseCursor` true))
    (:`then_1`
      (bind _playerstate (`self.PlayerState` :!label _label)
        (:`then`
          (bind _asbp_player_state (cast `/Game/Blueprint/AllLevel/System/BP_PlayerState` _playerstate))
          (`/Game/Blueprint/Gameplay/BP_HUD.InitializeScore` (`self.HUDRef`) _asbp_player_state))
        (:`else`
          (`KismetSystemLibrary.Delay` 0.5)
          (goto _label))))))

(event `self.OnPossessEvent`
  (params (InPawn :type "Pawn Object Reference"))
  (`parent.OnPossessEvent` InPawn)
  (bind _asbp_character (cast `/Game/Blueprint/Gameplay/Character/BP_Character` InPawn))
  (set `self.CharacterRef` _asbp_character)
  (`self.CLIENT_SetInputFocus`))

(event `self.ReceiveTick`
  (params (DeltaSeconds :type "Float (single-precision)"))
  (bind _cursor (`self.Cursor`))
  ;[1 1 1] Cursor UI Need to refactor
  (`parent.ReceiveTick` DeltaSeconds)
  (`|ExecutionSequence`
    (:`then_0`
      (`/Engine/EditorBlueprintResources/StandardMacros.IsValid` _cursor
        (:`Is Valid`
          (if (`self.GetIsAiming`)
            (`Widget.SetVisibility` _cursor "Visible")
            (else
              (`Widget.SetVisibility` _cursor "Hidden"))))))))

(event `CLIENT_SetInputFocus`
  (`|ExecutionSequence`
    (:`then_0`
      (`WidgetBlueprintLibrary.SetFocusToGameViewport`)
      (`WidgetBlueprintLibrary.SetInputMode_GameOnly` self)
      (set `self.bShowMouseCursor` false))
    (:`then_1`
      ;[1 1 1] Refactor To HUd
      (bind _returnvalue (`|CreateWidget` "/Game/UI/Gameplay/Player/Cursor_Widget.Cursor_Widget_C" self))
      (bind _output_get (set `self.Cursor` _returnvalue))
      (`UserWidget.AddToViewport` _output_get 0)
      (`Widget.SetVisibility` (`self.Cursor`) "Hidden"))))

(event `SERVER_AddToInventory`
  (params (Character :type "/Game/Blueprint/Gameplay/Character/BP_Character Object Reference") (UseableToAdd :type "Actor Class Reference") (WeaponToAdd :type "Actor Class Reference"))
  (bind (_bisweaponexist _weapon _powerup) (break `CharacterInvetory` (`Character_Base.Inventory` Character)))
  ;[1 1 1] Add Item at SERVER
  (`|ExecutionSequence`
    (:`then_0`
      (if (`KismetSystemLibrary.IsValidClass` UseableToAdd)
        (`KismetArrayLibrary.Array_Add` _powerup UseableToAdd)))
    (:`then_1`
      (if (`KismetSystemLibrary.IsValidClass` WeaponToAdd)
        (`KismetArrayLibrary.Array_Add` _weapon WeaponToAdd)))))

(event `SERVER_BuyItem`
  (params (BoughtItem :type "Weapon_Base Class Reference"))
  ;[1 1 1] BuyItem
  (`self.BuyItem` BoughtItem))

(fn `BuyItem`
  (params (WeaponClass :type "Weapon_Base Class Reference"))
  (locals (WeaponSpawned :type "Weapon_Base Object Reference"))
  (bind _characterref (`self.CharacterRef`))
  (`|ExecutionSequence`
    (:`then_0`
      (`/Engine/EditorBlueprintResources/ActorMacros.Switch Has Authority`
        (:`Authority`
          (bind _asbp_gameplay_gm (cast `/Game/Blueprint/AllLevel/System/BP_GameplayGM` (`GameplayStatics.GetGameMode`)))
          (bind _returnvalue (`MyGameMode_Base.SpawnWeapon` _asbp_gameplay_gm WeaponClass (0.0 0.0 0.0) (struct)))
          (set `local.WeaponSpawned` _returnvalue)
          (`Character_Base.AttachActorToMesh` _characterref _returnvalue)
          (`Character_Base.OnChangeWeapon` _characterref))
        (:`Remote`
          (`self.SERVER_BuyItem` WeaponClass))))))

(fn `CreateShopUI`
  (params (ItemToSell :type "Array of Actor Class Reference"))
  (returns (ShopWidgetRef :type "/Game/UI/Gameplay/Shop/Shop_Widget Object Reference"))
  (if (`self.IsLocalController`)
    (`self.ShopWidgetRef`
      (:`then`)
      (:`else`
        (bind _returnvalue (`|CreateWidget` "/Game/UI/Gameplay/Shop/Shop_Widget.Shop_Widget_C" null ItemToSell))
        (set `self.ShopWidgetRef` _returnvalue)
        (`UserWidget.AddToViewport` _returnvalue 0)
        (return (`self.ShopWidgetRef`))))))

(fn `OnRep_CharacterRef`
  (bind _hudref (`self.HUDRef`))
  (bind _characterref (`self.CharacterRef`))
  (`/Engine/EditorBlueprintResources/StandardMacros.IsValid` _hudref
    (:`Is Valid`
      (`/Engine/EditorBlueprintResources/StandardMacros.IsValid` _characterref
        (:`Is Valid`
          (`/Game/Blueprint/Gameplay/BP_HUD.OnInitializePlayer` _hudref _characterref))))))

(fn `UserConstructionScript`)