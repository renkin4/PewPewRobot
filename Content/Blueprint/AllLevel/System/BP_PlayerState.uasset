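; BP_PlayerState is a player state Blueprint that applies the player's saved name when play begins.
; On BeginPlay it caches BP_GameInstance and runs SetupName, which loads the save through that instance and caches it as MySaveInfo.
; If the saved PlayerName is non-empty and the owning controller is valid, it sets that name on the controller.
; Tick only calls the parent, and a team number debug print is left disconnected.
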(event `self.ReceiveTick`
  (params (DeltaSeconds :type "Float (single-precision)"))
  (`parent.ReceiveTick` DeltaSeconds))

(event `self.ReceiveBeginPlay`
  (`parent.ReceiveBeginPlay`)
  (bind _asbp_game_instance (cast `/Game/Blueprint/AllLevel/System/BP_GameInstance` (`GameplayStatics.GetGameInstance`)))
  (set `self.GameInstanceRef` _asbp_game_instance)
  (`self.SetupName`))

(fn `SetupName`
  (bind _returnvalue (`self.GetMyController`))
  (bind _playername (`/Game/Blueprint/AllLevel/System/MySaveInfo.GetAllData` (`self.SaveInfoRef`)))
  (bind _savegamedata (`/Game/Blueprint/AllLevel/System/BP_GameInstance.LoadGame` (`self.GameInstanceRef`)))
  (if (!= _savegamedata null)
    (bind _asmy_save_info (cast `/Game/Blueprint/AllLevel/System/MySaveInfo` _savegamedata))
    (set `self.SaveInfoRef` _asmy_save_info)
    (if (`KismetStringLibrary.NotEqual_StrStr` _playername)
      (`/Engine/EditorBlueprintResources/StandardMacros.IsValid` _returnvalue
        (:`Is Valid`
          (`AdvancedSessionsLibrary.SetPlayerName` _returnvalue _playername))))))

(fn `UserConstructionScript`)