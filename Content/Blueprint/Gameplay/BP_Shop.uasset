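; BP_Shop is a shop actor that opens a shop UI for the player.
; Its box overlap binds and unbinds a handler on BP_Character's OnNearShop delegate as the character enters and leaves.
; When that delegate fires, player controller 0 creates the UI from the ItemsToSell actor class.
; The shop then shows the cursor and switches to UI-only input focused on the widget, with the mouse locked.
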(event `self.Box.OnComponentBeginOverlap`
  (params (OverlappedComponent :type "PrimitiveComponent Object Reference") (OtherActor :type "Actor Object Reference") (OtherComp :type "PrimitiveComponent Object Reference") (OtherBodyIndex :type Integer) (bFromSweep :type Boolean) (SweepResult :type "HitResult Structure (by ref)"))
  (bind _asbp_character (cast `/Game/Blueprint/Gameplay/Character/BP_Character` OtherActor))
  (add `/Game/Blueprint/Gameplay/Character/BP_Character.DelegateOnNearShop` _asbp_character (delegate `NearShopDelegate`)))

(event `NearShopDelegate`
  (bind _returnvalue (`GameplayStatics.GetPlayerController` 0))
  (bind _asbp_player_controller (cast `/Game/Blueprint/AllLevel/System/BP_PlayerController` _returnvalue))
  (bind _shopwidgetref (`/Game/Blueprint/AllLevel/System/BP_PlayerController.CreateShopUI` _asbp_player_controller (`.ActorClass` (break `ItemsToSell` (`self.ItemsToSell`)))))
  (set `PlayerController.bShowMouseCursor` true _returnvalue)
  (`WidgetBlueprintLibrary.SetInputMode_UIOnlyEx` _returnvalue _shopwidgetref "LockAlways"))

(event `self.Box.OnComponentEndOverlap`
  (params (OverlappedComponent :type "PrimitiveComponent Object Reference") (OtherActor :type "Actor Object Reference") (OtherComp :type "PrimitiveComponent Object Reference") (OtherBodyIndex :type Integer))
  (bind _asbp_character (cast `/Game/Blueprint/Gameplay/Character/BP_Character` OtherActor))
  (remove `/Game/Blueprint/Gameplay/Character/BP_Character.DelegateOnNearShop` _asbp_character (delegate `NearShopDelegate`)))

(fn `UserConstructionScript`)