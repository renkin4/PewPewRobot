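; Throwable stun grenade loot item that stuns characters within a radius when its sphere first overlaps after use.
; Use multicasts projectile and collision setup, then binds detonation to the overlap delegate.
; Detonation runs once, squared-distance checking all Characters: AI are stunned through their controller, others by multicast to BP_Character.
; It then multicasts a debug-sphere placeholder effect and has the game state destroy the grenade.
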(event `MUTLICAST_InitializationOnUse`
  (bind _projectilemovement (`self.ProjectileMovement`))
  ;[1 1 1] Initialize On USe
  (set `ProjectileMovementComponent.MaxSpeed` (`ProjectileMovementComponent.InitialSpeed` _projectilemovement) _projectilemovement)
  (set `ProjectileMovementComponent.ProjectileGravityScale` 1.0 _projectilemovement)
  (`PrimitiveComponent.SetCollisionResponseToChannel` (`self.GrenadeMesh`) "ECC_GameTraceChannel4" "ECR_Ignore"))

(event `BindOnOverlapDelegate`
  (bind _distanceawaysq (`self.DistanceAwaySq`))
  ;[1 1 1] On Use
  (`/Engine/EditorBlueprintResources/StandardMacros.DoOnce` false
    (:`Completed`
      (`|ExecutionSequence`
        (:`then_0`
          (bind _outactors (`GameplayStatics.GetAllActorsOfClass` "/Script/Engine.Character"))
          (for _array_element _outactors
            (if (!= _array_element self)
              (if (<= (`KismetMathLibrary.VSizeSquared` (- (`self.K2_GetActorLocation`) (`self.K2_GetActorLocation` _array_element))) (* _distanceawaysq _distanceawaysq))
                (if (`KismetMathLibrary.ClassIsChildOf` (`GameplayStatics.GetObjectClass` _array_element) "/Script/Sem6.AICharacter")
                  (`MyAIController.SetStunAI` (cast `/Game/Blueprint/Gameplay/AI/BP_AIController` (`Pawn.GetController` _array_element) :!pure true) true (`self.StunDuration`))
                  (else
                    (`self.MULTICAST_StunCharacter` _array_element (`self.StunDuration`))))))))
        (:`then_1`
          (`self.MULTICAST_FXSimulate`)
          (`self.DestroySelf` self))))))

(event `self.OnUseAction`
  ;[1 1 1] On Use
  (`self.MUTLICAST_InitializationOnUse`)
  (add `self.OnOverlapDelegate` (delegate `BindOnOverlapDelegate`)))

(event `self.Sphere.OnComponentBeginOverlap`
  (params (OverlappedComponent :type "PrimitiveComponent Object Reference") (OtherActor :type "Actor Object Reference") (OtherComp :type "PrimitiveComponent Object Reference") (OtherBodyIndex :type Integer) (bFromSweep :type Boolean) (SweepResult :type "HitResult Structure (by ref)"))
  (`self.OnOverlapDelegate`))

(event `DestroySelf`
  (params (ActorToDestroy :type "Actor Object Reference"))
  ;[1 1 1] Destroy Self (Run On Server)
  (`MyGameState_Base.DestroyingActor` (cast `/Game/Blueprint/AllLevel/System/BP_GameplayGS` (`GameplayStatics.GetGameState`) :!pure true) ActorToDestroy))

(event `MULTICAST_StunCharacter`
  (params (Character :type "Object Object Reference") (StunDuration :type "Float (double-precision)"))
  (bind _asbp_character (cast `/Game/Blueprint/Gameplay/Character/BP_Character` Character))
  (`Character_Base.StunPlayer` _asbp_character StunDuration))

(event `MULTICAST_FXSimulate`
  ;[1 1 1] Simulate Particle ETC
  (`KismetSystemLibrary.DrawDebugSphere` (`self.K2_GetActorLocation`) (`self.DistanceAwaySq`) 12 (struct :`R` 10.0 :`G` 1.0 :`B` 5.0 :`A` 1.0) 1.5 10.0))

(fn `UserConstructionScript`)