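; Player start that creates a spawn point at its position and registers it as a player's spawn location.
; On BeginPlay it asks BP_GameplayGM to spawn a BP_SpawnPoint slightly below itself, stores it and sets itself as that point's owner.
; It then polls every half second until its player controller is valid, and passes the spawn point to that controller's BP_PlayerState.
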(event `self.ReceiveBeginPlay`
  (bind _returnvalue (`self.GetPController`))
  (bind (_returnvalue_location _returnvalue_rotation) (`KismetMathLibrary.BreakTransform` (`self.GetTransform`)))
  (`|ExecutionSequence`
    (:`then_0`
      (bind _asbp_gameplay_gm (cast `/Game/Blueprint/AllLevel/System/BP_GameplayGM` (`GameplayStatics.GetGameMode`)))
      (bind _output_get (set `self.GameModeRef` _asbp_gameplay_gm))
      (bind _returnvalue_2 (`MyGameMode_Base.SpawnBase` _output_get "/Game/Blueprint/Gameplay/SpawnPoint/BP_SpawnPoint.BP_SpawnPoint_C" (+ _returnvalue_location (0.0 0.0 -80.0)) _returnvalue_rotation))
      (`self.SetSpawnPointBase` _returnvalue_2)
      (`SpawnPoint_Base.SetMyOwner` (`self.SpawnPointBase`) self)
      (`/Engine/EditorBlueprintResources/StandardMacros.IsValid` _returnvalue :!label _label
        (:`Is Valid`
          (`PlayerState_Base.SetSpawnLocation` (cast `/Game/Blueprint/AllLevel/System/BP_PlayerState` (`Controller.PlayerState` _returnvalue) :!pure true) (`self.SpawnPointBase`)))
        (:`Is Not Valid`
          (`KismetSystemLibrary.Delay` 0.5)
          (goto _label))))
    (:`then_1`)))

(fn `UserConstructionScript`)