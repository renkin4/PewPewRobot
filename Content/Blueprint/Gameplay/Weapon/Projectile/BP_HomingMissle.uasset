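; Homing missile projectile that explodes on overlapping an actor whose class differs from its owner's, then destroys itself.
; The blast checks every Character within Radius by squared distance, stunning AICharacters through BP_AIController for StunTimer and applying damage to the others.
; It spawns an explosion emitter at impact; no homing logic appears in these graphs.
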(event `self.ReceiveBeginPlay`
  (`parent.ReceiveBeginPlay`))

(event `self.ReceiveTick`
  (params (DeltaSeconds :type "Float (single-precision)"))
  (`parent.ReceiveTick` DeltaSeconds))

(event `self.Sphere.OnComponentBeginOverlap`
  (params (OverlappedComponent :type "PrimitiveComponent Object Reference") (OtherActor :type "Actor Object Reference") (OtherComp :type "PrimitiveComponent Object Reference") (OtherBodyIndex :type Integer) (bFromSweep :type Boolean) (SweepResult :type "HitResult Structure (by ref)"))
  (if (!= (`GameplayStatics.GetObjectClass` OtherActor) (`GameplayStatics.GetObjectClass` (`self.GetOwner`)))
    (bind _outactors (`GameplayStatics.GetAllActorsOfClass` "/Script/Engine.Character"))
    (for _array_element _outactors
      (if (<= (`KismetMathLibrary.VSizeSquared` (- (`self.K2_GetActorLocation` _array_element) (`self.K2_GetActorLocation`))) (* (`self.Radius`) (`self.Radius`)))
        (if (`KismetMathLibrary.ClassIsChildOf` (`GameplayStatics.GetObjectClass` _array_element) "/Script/Sem6.AICharacter")
          (bind _asbp_aicontroller (cast `/Game/Blueprint/Gameplay/AI/BP_AIController` (`AIBlueprintHelperLibrary.GetAIController` _array_element)))
          (`MyAIController.SetStunAI` _asbp_aicontroller true (`self.StunTimer`))
          (else
            (`GameplayStatics.ApplyDamage` _array_element 1.0 null self "/Game/Blueprint/Gameplay/DamageType/BP_HomingMissle.BP_HomingMissle_C")))))
    (`GameplayStatics.SpawnEmitterAtLocation` "/Game/StarterContent/Particles/P_Explosion.P_Explosion" (`self.K2_GetActorLocation`) (`self.K2_GetActorRotation`))
    (`self.K2_DestroyActor`)))

(fn `UserConstructionScript`
  (`parent.UserConstructionScript`))