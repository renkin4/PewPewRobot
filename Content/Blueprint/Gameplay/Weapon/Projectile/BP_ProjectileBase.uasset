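; Base projectile that configures itself from the BP_RocketLauncher that owns it.
; On BeginPlay, Initiliaze casts the owner to that launcher and copies shot interval, radial radius, stun delay and stamina cost from its MyStats into local variables.
; It then applies the launcher's velocity and gravity to ProjectileMovement's initial speed, max speed and gravity scale.
; The graphs shown contain no impact, damage or stun logic.
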(event `self.ReceiveBeginPlay`
  (`self.Initiliaze`))

(fn `Initiliaze`
  (bind _projectilemovement (`self.ProjectileMovement`))
  (bind _asbp_rocket_launcher (cast `/Game/Blueprint/Gameplay/Weapon/BP_RocketLauncher` (`self.GetOwner`) :!pure true))
  (bind _projectilevelocity (`Weapon_Base.ProjectileVelocity` _asbp_rocket_launcher))
  (bind (_shotsbetweeninterval _radialradius _stundelayduration _staminacost) (break `WeaponStats` (`Weapon_Base.MyStats` _asbp_rocket_launcher)))
  (`|ExecutionSequence`
    (:`then_0`
      (set `self.ShotInterval` _shotsbetweeninterval)
      (set `self.Radius` _radialradius)
      (set `self.StunTimer` _stundelayduration)
      (set `self.StaminaCost` _staminacost))
    (:`then_1`
      (set `ProjectileMovementComponent.MaxSpeed` _projectilevelocity _projectilemovement)
      (set `ProjectileMovementComponent.InitialSpeed` _projectilevelocity _projectilemovement)
      (set `ProjectileMovementComponent.ProjectileGravityScale` (`Weapon_Base.ProjectileGravity` _asbp_rocket_launcher) _projectilemovement))))

(fn `UserConstructionScript`)