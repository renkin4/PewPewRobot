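; Player character Blueprint adding camera pitch limits, shop and debug inputs, and throwable power-up use.
; On loot use, a client event computes spawn transform from control rotation when targeting, otherwise a fixed upward pitch.
; The server then has the game mode spawn the first inventory power-up, triggers it and removes it.
; Timeline and interpolation smooth displayed health and stamina; the self-damage event's only call is unwired.
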(event `InputAction|Shop`
  (params (Key :type "Key Structure" :default "AnyKey"))
  (:`Pressed`
    (`self.DelegateOnNearShop`)))

(event `SERVER_DealDamage`
  (`GameplayStatics.ApplyDamage` self 5.0 null self "/Script/Engine.DamageType"))

(event `self.OnRep_Health`
  ;[1 1 1] Asthethic
  (bind (_direction _healthtimelinespeed) (`Timeline|HealthTimeline` :!via `PlayFromStart`)
    (:`Update`
      (set `self.LocalHealth` (`KismetMathLibrary.Lerp` (`self.LocalHealth`) (`self.Health`) _healthtimelinespeed)))))

(event `InputAction|Debug`
  (params (Key :type "Key Structure" :default "AnyKey"))
  (:`Pressed`
    (`GameplayStatics.OpenLevel` "Debug")))

(event `self.ReceiveBeginPlay`
  (bind _returnvalue (`GameplayStatics.GetPlayerCameraManager` 0))
  ;[1 1 1] BeginPlay
  (`parent.ReceiveBeginPlay`)
  (set `PlayerCameraManager.ViewPitchMax` (`self.MaxPitch`) _returnvalue)
  (set `PlayerCameraManager.ViewPitchMin` (`self.MinPitch`) _returnvalue)
  (add `self.OnUseLootableDelegate` (delegate `OnUseLootableDelgateBind`)))

(event `OnUseLootableDelgateBind`
  ;[1 1 1] BeginPlay
  (`|ExecutionSequence`
    (:`then_0`
      (if (`KismetArrayLibrary.Array_IsValidIndex` (`.PowerUp` (break `CharacterInvetory` (`self.Inventory`))))
        ;;[1 1 1] TODO only for Throwable
        (`self.CLIENT_CalculateRotationForThrowable`)))))

(event `SERVER_SpawnThrowable`
  (params (Location :type "Vector Structure") (Rotation :type "Rotator Structure"))
  ;[1 1 1] TODO Refactor
  (bind _asbp_gameplay_gm (cast `/Game/Blueprint/AllLevel/System/BP_GameplayGM` (`GameplayStatics.GetGameMode`)))
  (bind _returnvalue (`MyGameMode_Base.SpawnLoot` _asbp_gameplay_gm (castclass `Loot_Base` (`|GetArrayItem` (`.PowerUp` (break `CharacterInvetory` (`self.Inventory`)))) :!pure true) Location Rotation))
  (`/Engine/EditorBlueprintResources/StandardMacros.IsValid` _returnvalue
    (:`Is Valid`
      (`Loot_Base.OnUseAction` _returnvalue)
      (`KismetArrayLibrary.Array_Remove` (`.PowerUp` (break `CharacterInvetory` (`self.Inventory`)))))))

(event `self.ReceiveTick`
  (params (DeltaSeconds :type "Float (single-precision)"))
  (`parent.ReceiveTick` DeltaSeconds)
  (set `self.AsthethicStaminaVal` (`KismetMathLibrary.FInterpTo` (`self.AsthethicStaminaVal`) (`self.GetStaminaVal`) DeltaSeconds (`self.StaminaInterpSpeed`))))

(event `self.ReceiveEndPlay`
  (params (EndPlayReason :type "EEndPlayReason Enum" :default "Destroyed"))
  (bind _itemselectionwidget (`self.ItemSelectionWidget`))
  (switch `EEndPlayReason` EndPlayReason
    (:`Destroyed`
      (if (`KismetSystemLibrary.IsValid` _itemselectionwidget)
        (`Widget.RemoveFromParent` _itemselectionwidget)))))

(event `CLIENT_CalculateRotationForThrowable`
  (bind (_rotation _actorlocation) (`self.CalculateRotationForThrowable`))
  (`self.SERVER_SpawnThrowable` _actorlocation _rotation))

(fn `CalculateRotationForThrowable`
  (returns (Rotation :type "Rotator Structure") (ActorLocation :type "Vector Structure"))
  (locals (SpawnThrowableRotation :type "Rotator Structure" :default (struct)))
  (bind (_returnvalue_roll _returnvalue_pitch _returnvalue_yaw) (`KismetMathLibrary.BreakRotator` (`self.K2_GetActorRotation`)))
  (bind _returnvalue (`self.K2_GetActorLocation`))
  (if (`self.GetIsTargetting`)
    (set `local.SpawnThrowableRotation` (`KismetMathLibrary.FindLookAtRotation` _returnvalue (+ (* (`KismetMathLibrary.GetForwardVector` (`self.GetControlRotation`)) 2000) _returnvalue)))
    (else
      (set `local.SpawnThrowableRotation` (`KismetMathLibrary.MakeRotator` _returnvalue_roll 25.0 _returnvalue_yaw))))
  (return (`local.SpawnThrowableRotation`) (+ (+ (`self.K2_GetActorLocation`) (`KismetMathLibrary.MakeVector` 0.0 0.0 (`self.BaseEyeHeight`))) (* (`KismetMathLibrary.GetForwardVector` (`self.K2_GetActorRotation`)) 150))))

(fn `UserConstructionScript`)